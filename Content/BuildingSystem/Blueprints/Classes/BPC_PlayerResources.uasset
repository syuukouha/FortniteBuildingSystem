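; Player resources component for the building system that tracks the selected resource and keeps its UI in sync.
; On initialization it has the player's main widget generate resource widgets, fills in each amount from the Resources map and highlights the current selection.
; Selection cycles through the map's keys with wraparound, refreshing the main widget and firing OnResourceSwitched.
; Amount updates also refresh the current-resource display when that resource is selected and the player is in a specific state.
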(event `OnResourceSwitched`)

(event `InitializeManager`
  (params (Player :type "/Game/ThirdPersonBP/Blueprints/ThirdPersonCharacter Object Reference"))
  (`/Engine/EditorBlueprintResources/StandardMacros.IsValid` Player
    (:`Is Valid`
      (bind _output_get (set `self.Ref_Player` Player))
      (set `self.Initialized?` true)
      (bind _createdwidgets (`/Game/BuildingSystem/Widgets/WBP_Main.GenerateResourceWidgets` (`/Game/ThirdPersonBP/Blueprints/ThirdPersonCharacter.Ref_MainWidget` _output_get) self))
      (set `self.ResourceWidgets` _createdwidgets)
      (bind _keys (`BlueprintMapLibrary.Map_Keys` (`self.Resources`)))
      (for _array_element _keys
        (`self.UpdateResourceDisplay` _array_element))
      (`self.SelectCurrentResource`))))

(event `self.UpdateResourceDisplay`
  (params (Resource :type "/Game/BuildingSystem/Blueprints/Classes/BP_Master_Resource Class Reference"))
  (bind (_success_ _widget) (`self.GetWidgetForResource` Resource))
  (if (`self.Initialized?`)
    (if _success_
      (`TextBlock.SetText` (`/Game/BuildingSystem/Widgets/WBP_Resource.Amount` _widget) (`KismetTextLibrary.Conv_IntToText` (`self.GetResource` Resource) false false))
      (if (and (== (`self.GetSelectedResource`) Resource) (`|EnumEquality` (`/Game/ThirdPersonBP/Blueprints/ThirdPersonCharacter.State` (`self.Ref_Player`)) "NewEnumerator1"))
        (`/Game/BuildingSystem/Widgets/WBP_Main.UpdateCurrentResource` (`/Game/ThirdPersonBP/Blueprints/ThirdPersonCharacter.Ref_MainWidget` (`self.Ref_Player`)) self)))))

(fn `GetCurrentlySelectedWidget`
  (returns (Widget :type "/Game/BuildingSystem/Widgets/WBP_Resource Object Reference"))
  (return (`.Widget` (`self.GetWidgetForResource` (`self.GetSelectedResource`)))))

(fn `GetSelectedIndex`
  (returns (SelectedResourceIndex :type Integer))
  (return (`self.SelectedResourceIndex`)))

(fn `GetSelectedResource`
  (returns (Output :type "/Game/BuildingSystem/Blueprints/Classes/BP_Master_Resource Class Reference"))
  (bind _keys (`BlueprintMapLibrary.Map_Keys` (`self.Resources`)))
  (return (`|GetArrayItem` _keys (`self.SelectedResourceIndex`))))

(fn `GetWidgetForResource`
  (params (Resource :type "/Game/BuildingSystem/Blueprints/Classes/BP_Master_Resource Class Reference"))
  (returns (`Success?` :type Boolean) (Widget :type "/Game/BuildingSystem/Widgets/WBP_Resource Object Reference"))
  (locals (LocalResourceWidget :type "/Game/BuildingSystem/Widgets/WBP_Resource Object Reference"))
  (bind _localresourcewidget (`local.LocalResourceWidget`))
  (for _array_element (`self.ResourceWidgets`)
    (if (== (`/Game/BuildingSystem/Widgets/WBP_Resource.Resource` _array_element) Resource)
      (set `local.LocalResourceWidget` _array_element)
      (break)))
  (`/Engine/EditorBlueprintResources/StandardMacros.IsValid` _localresourcewidget
    (:`Is Valid`
      (return true _localresourcewidget))
    (:`Is Not Valid`
      (return false null))))

(fn `SelectCurrentResource`
  (`/Game/BuildingSystem/Widgets/WBP_Resource.SelectResource` (`self.GetCurrentlySelectedWidget`) true false))

(fn `SelectNextResource`
  (bind _selectedresourceindex (`self.SelectedResourceIndex`))
  (`/Game/BuildingSystem/Widgets/WBP_Resource.SelectResource` (`self.GetCurrentlySelectedWidget`) false false)
  (bind _keys (`BlueprintMapLibrary.Map_Keys` (`self.Resources`)))
  (set `self.SelectedResourceIndex` (`KismetMathLibrary.SelectInt` (+ _selectedresourceindex 1) 0 (< _selectedresourceindex (`KismetArrayLibrary.Array_LastIndex` _keys))))
  (`self.SelectCurrentResource`)
  (`/Game/BuildingSystem/Widgets/WBP_Main.UpdateCurrentResource` (`/Game/ThirdPersonBP/Blueprints/ThirdPersonCharacter.Ref_MainWidget` (`self.Ref_Player`)) self)
  (`self.OnResourceSwitched`))
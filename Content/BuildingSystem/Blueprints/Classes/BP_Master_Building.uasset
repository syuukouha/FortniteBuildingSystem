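; Master building actor that starts as a tinted ghost with a build widget and becomes a solid, health-tracked structure once built.
; The selected resource class drives ghost color, final material and the version data for max health and build time.
; On build, it blocks all channels, swaps the widget for a health bar, and a looping timer raises health until full.
; A delay also ends construction as a fallback, clearing the timer.
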(event `self.ReceiveBeginPlay`
  (bind _buildingmesh (`self.BuildingMesh`))
  (bind _returnvalue (`PrimitiveComponent.CreateDynamicMaterialInstance` _buildingmesh 0 (`PrimitiveComponent.GetMaterial` _buildingmesh 0) "None"))
  (set `self.DynamicMaterial` _returnvalue)
  (`self.UpdateGhostMaterial`)
  (bind _aswbp_build (cast `/Game/BuildingSystem/Widgets/WBP_Build` (`WidgetComponent.GetUserWidgetObject` (`self.BuildWidget`))))
  (set `self.Ref_BuildWidget` _aswbp_build)
  (bind _aswbp_building_health_bar (cast `/Game/BuildingSystem/Widgets/WBP_BuildingHealthBar` (`WidgetComponent.GetUserWidgetObject` (`self.HealthBar`))))
  (set `self.Ref_HealthBar` _aswbp_building_health_bar)
  (`/Game/BuildingSystem/Widgets/WBP_Build.Update` (`self.Ref_BuildWidget`) (`BlueprintMapLibrary.Map_Find` (`self.ResourceVersions`) (`self.Resource`)) (`self.Resource`))
  (`/Game/BuildingSystem/Blueprints/Classes/BPC_BuildingStats.InitializeManager` (`self.BPC_BuildingStats`) self)
  (`SceneComponent.SetVisibility` (`self.BuildWidget`) true false))

(event `SetCanBeBuilt`
  (params (NewParam :type Boolean))
  (bind _output_get (set `self.CanBeBuilt?` NewParam))
  (`/Game/BuildingSystem/Widgets/WBP_Build.SetCanBeBuilt` (`self.Ref_BuildWidget`) _output_get))

(event `OnBuild`
  (params (Resource :type "/Game/BuildingSystem/Blueprints/Classes/BP_Master_Resource Class Reference"))
  (bind _bpc_buildingstats (`self.BPC_BuildingStats`))
  (bind _buildingmesh (`self.BuildingMesh`))
  (bind (_requiredamount _buildingtime _maxbuildinghealth) (break `/Game/BuildingSystem/Blueprints/Structures/S_BuildingResourceVersion` (`BlueprintMapLibrary.Map_Find` (`self.ResourceVersions`) Resource)))
  (if (`KismetSystemLibrary.IsValidClass` Resource)
    (set `self.Built?` true)
    (`PrimitiveComponent.SetCollisionResponseToAllChannels` _buildingmesh "ECR_Block")
    (`PrimitiveComponent.SetMaterial` _buildingmesh 0 (`.BuildingMaterial_11_1B62C7874186A4908A7C86945B493DFA` (break `/Game/BuildingSystem/Blueprints/Structures/S_ResourceData` (defaults `/Game/BuildingSystem/Blueprints/Classes/BP_Master_Building` Resource))))
    (`ActorComponent.K2_DestroyComponent` (`self.BuildWidget`))
    (`/Game/BuildingSystem/Blueprints/Classes/BPC_BuildingStats.SetMaxStatValue` _bpc_buildingstats "NewEnumerator2" _maxbuildinghealth false)
    (`/Game/BuildingSystem/Blueprints/Classes/BPC_Master_StatManager.SetStat` _bpc_buildingstats "NewEnumerator2" 0 false)
    (set `self.BuildingTime` _buildingtime)
    (`/Game/BuildingSystem/Widgets/WBP_BuildingHealthBar.InitializeBar` (`self.Ref_HealthBar`) (`/Game/BuildingSystem/Blueprints/Classes/BPC_BuildingStats.GetMaxHealth` _bpc_buildingstats))
    (`SceneComponent.SetVisibility` (`self.HealthBar`) true false)
    (bind _returnvalue (`KismetSystemLibrary.K2_SetTimerDelegate` (delegate `BuildingTick`) (`self.Interval`) true))
    (set `self.BuildingTimerHandle` _returnvalue)
    (`KismetSystemLibrary.Delay` (+ (`self.BuildingTime`) (`self.Interval`)))
    (`self.OnBuildingEnd`)))

(event `BuildingTick`
  (bind _bpc_buildingstats (`self.BPC_BuildingStats`))
  (`/Game/BuildingSystem/Blueprints/Classes/BPC_Master_StatManager.ModifyStat` _bpc_buildingstats "NewEnumerator2" (`KismetMathLibrary.FCeil` (/ (`KismetMathLibrary.Conv_IntToDouble` (`/Game/BuildingSystem/Blueprints/Classes/BPC_BuildingStats.GetMaxHealth` (`self.BPC_BuildingStats`))) (`KismetMathLibrary.Conv_IntToDouble` (`KismetMathLibrary.FFloor` (/ (`self.BuildingTime`) (`self.Interval`)))))))
  (if (== (`/Game/BuildingSystem/Blueprints/Classes/BPC_Master_StatManager.GetStat` _bpc_buildingstats "NewEnumerator2") (`/Game/BuildingSystem/Blueprints/Classes/BPC_BuildingStats.GetMaxHealth` _bpc_buildingstats))
    (`self.OnBuildingEnd`)))

(event `OnBuildingEnd`
  (if (`KismetSystemLibrary.K2_IsValidTimerHandle` (`self.BuildingTimerHandle`))
    (`KismetSystemLibrary.K2_ClearAndInvalidateTimerHandle` (`self.BuildingTimerHandle`))
    (`/Game/BuildingSystem/Widgets/WBP_BuildingHealthBar.SetState` (`self.Ref_HealthBar`) "NewEnumerator1")))

(fn `ChangeResource`
  (params (NewResource :type "/Game/BuildingSystem/Blueprints/Classes/BP_Master_Resource Class Reference"))
  (bind _resource (`self.Resource`))
  (if (and (`KismetSystemLibrary.IsValidClass` NewResource) (!= NewResource (`self.Resource`)))
    (set `self.Resource` NewResource)
    (`self.UpdateGhostMaterial`)
    (`/Game/BuildingSystem/Widgets/WBP_Build.Update` (`self.Ref_BuildWidget`) (`BlueprintMapLibrary.Map_Find` (`self.ResourceVersions`) _resource) _resource)))

(fn `UpdateGhostMaterial`
  (`MaterialInstanceDynamic.SetVectorParameterValue` (`self.DynamicMaterial`) "Color" (`.GhostBuildingColor_8_5F1D84E44F10A764EDB585AE7E6C12E4` (break `/Game/BuildingSystem/Blueprints/Structures/S_ResourceData` (defaults `/Game/BuildingSystem/Blueprints/Classes/BP_Master_Building` (`self.Resource`))))))

(fn `UserConstructionScript`)
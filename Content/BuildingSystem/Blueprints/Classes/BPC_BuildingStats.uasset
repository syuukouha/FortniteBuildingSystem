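; Building stats component that stores a building's stats as a map of min, max and current values.
; InitializeManager caches the owning building and runs stat setup.
; SetMaxStatValue rewrites an existing stat's maximum, clamps its current value to the new range and optionally fires UpdateStat.
; UpdateStat refreshes the building's health bar when health changes and the building is in player sight.
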(event `InitializeManager`
  (params (Building :type "/Game/BuildingSystem/Blueprints/Classes/BP_Master_Building Object Reference"))
  (`/Engine/EditorBlueprintResources/StandardMacros.IsValid` Building
    (:`Is Valid`
      (set `self.Ref_Building` Building)
      (`self.SetUpStats`))))

(event `self.UpdateStat`
  (params (Stat :type "/Game/BuildingSystem/Blueprints/Enums/E_Stats Enum" :default "NewEnumerator0"))
  (if (and (`|EnumEquality` Stat "NewEnumerator2") (`/Game/BuildingSystem/Blueprints/Classes/BP_Master_Building.InPlayerSight?` (`self.Ref_Building`)))
    (`/Game/BuildingSystem/Widgets/WBP_BuildingHealthBar.UpdateHealth` (`/Game/BuildingSystem/Blueprints/Classes/BP_Master_Building.Ref_HealthBar` (`self.Ref_Building`)) (`self.GetStat` "NewEnumerator2"))))

(fn `GetMaxHealth`
  (returns (MaxValue :type Integer))
  (return (`.MaxValue_5_B2376D8F42F80A72CFDC71AD198EBB7E` (break `/Game/BuildingSystem/Blueprints/Structures/S_StatValue` (`.StatValue` (`self.GetStat` "NewEnumerator2"))))))

(fn `SetMaxStatValue`
  (params (Stat :type "/Game/BuildingSystem/Blueprints/Enums/E_Stats Enum" :default "NewEnumerator0") (NewParam :type Integer) (`Update?` :type Boolean))
  (locals (LocalStat :type "/Game/BuildingSystem/Blueprints/Enums/E_Stats Enum" :default "NewEnumerator0") (LocalValue :type Integer) (LocalUpdate :type Boolean))
  (bind _localstat (`local.LocalStat`))
  (bind _localvalue (`local.LocalValue`))
  (bind (_currentvalue _statvalue) (`self.GetStat` (`local.LocalStat`)))
  (bind _minvalue (break `/Game/BuildingSystem/Blueprints/Structures/S_StatValue` _statvalue))
  (set `local.LocalStat` Stat)
  (set `local.LocalValue` NewParam)
  (set `local.LocalUpdate` `Update?`)
  (bind _keys (`BlueprintMapLibrary.Map_Keys` (`self.Stats`)))
  (if (and (`KismetArrayLibrary.Array_Contains` _keys _localstat) (`|EnumInequality` _localstat "NewEnumerator0"))
    (`BlueprintMapLibrary.Map_Add` (`self.Stats`) (`local.LocalStat`) (make `/Game/BuildingSystem/Blueprints/Structures/S_StatValue` _minvalue _localvalue (`KismetMathLibrary.Clamp` _currentvalue _minvalue _localvalue)))
    (if (`local.LocalUpdate`)
      (`self.UpdateStat` (`local.LocalStat`)))))